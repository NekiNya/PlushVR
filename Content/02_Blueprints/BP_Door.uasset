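; BP_Door is a door actor that swings open or shut when its Interact event is called.
; A normal interaction works once: it sets Open, clears Tags and plays the DoorAnim timeline, which drives the yaw of the Empty component.
; A Special interaction also works once, setting BlockDoor and reversing the timeline to swing the door back.
; Neither flag is reset here, and BlockDoor does not gate normal opening.
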(event EventBeginPlay)

(event Collision|EventActorBeginOverlap
  (params (OtherActor :type Actor%20Object%20Reference)))

(event EventTick
  (params (DeltaSeconds :type Float%20%28single-precision%29)))

(event EventInteract
  (params (Special :type Boolean))
  (if Special
    (if (not (Variables|Default|GetBlockDoor))
      (Variables|Default|SetBlockDoor true)
      ;[1 1 1] Intercalar Puerta
      (bind _rotation (Timeline|DoorAnim Reverse)
        (:Update
          (Transformation|SetRelativeRotation (Variables|Default|GetEmpty) (Math|Rotator|MakeRotator 0.0 0.0 _rotation) false false))))
    (elif (not (Variables|Default|GetOpen))
      (Variables|Default|SetOpen true)
      (Utilities|Array|Clear (Variables|Actor|GetTags))
      (Timeline|DoorAnim Play))))

(fn ConstructionScript)